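; Enemy character Blueprint for SpaceBlaster that handles its own death through health, combat and item-dropper components.
; When a health change leaves it dead, it plays a death sound, releases the trigger, detaches its controller, drops its weapon and attempts an item drop.
; It then disables capsule collision, switches the mesh to the Ragdoll collision profile, and destroys the weapon and itself after a short delay.
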(event `self.BP_HealthComponent.OnHealthChanged`
  (params (InstigatorActor :type "Actor Object Reference") (OwningComponent :type "/Game/SpaceBlaster/Core/Components/BP_HealthComponent Object Reference") (NewHealth :type "Float (double-precision)"))
  (bind _bp_combatcomponent (`self.BP_CombatComponent`))
  (if (not (`/Game/SpaceBlaster/Core/Components/BP_HealthComponent.IsAlive` OwningComponent))
    (`GameplayStatics.PlaySoundAtLocation` (`self.DeathSound`) (`self.K2_GetActorLocation`) (struct) 1.0 1.0 0.0 null null null null)
    (`/Game/SpaceBlaster/Combat/BP_CombatComponent.ReleaseTrigger` _bp_combatcomponent)
    (`self.DetachFromControllerPendingDestroy`)
    (`/Game/SpaceBlaster/Combat/BP_CombatComponent.DropWeapon` _bp_combatcomponent)
    (`/Game/SpaceBlaster/BP_ItemDropper.AttempItemDrop` (`self.BP_ItemDropper`))
    (`PrimitiveComponent.SetCollisionEnabled` (`self.CapsuleComponent`) "NoCollision")
    (`PrimitiveComponent.SetCollisionProfileName` (`self.Mesh`) "Ragdoll" true)
    (`KismetSystemLibrary.Delay` 5.0)
    (`self.K2_DestroyActor` (`/Game/SpaceBlaster/Combat/BP_CombatComponent.CurrentWeapon` _bp_combatcomponent))
    (`self.K2_DestroyActor`)))

(fn `UserConstructionScript`)