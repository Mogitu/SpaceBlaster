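; BP_PlayerCharacter is the player-controlled character in SpaceBlaster, handling movement, firing, interaction and death.
; Axis inputs feed AddMovementInput along world X and Y, while Fire and Interact presses delegate to CombatComponent and BPInteractionComponent.
; HealthComponent's OnHealthChanged calls Kill, which destroys the current weapon and then the character once health reaches zero or below.
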(event `self.HealthComponent.OnHealthChanged`
  (params (NewHealth :type "Float (double-precision)"))
  ;[0.2705 0.88 1] Component event handling
  (`self.Kill` NewHealth))

(event `InputAxis|MoveForward`
  (params (AxisValue :type "Float (single-precision)"))
  ;[0.4625 0.2874 1] Player Movement
  (`self.AddMovementInput` (`KismetMathLibrary.MakeVector` AxisValue)))

(event `InputAxis|MoveRight`
  (params (AxisValue :type "Float (single-precision)"))
  ;[0.4625 0.2874 1] Player Movement
  (`self.AddMovementInput` (`KismetMathLibrary.MakeVector` 0.0 AxisValue)))

(event `InputAction|Fire`
  (params (Key :type "Key Structure"))
  ;[1 0.1042 0.1042] Player actions
  (:`Pressed`
    (`/Game/SpaceBlaster/Combat/BP_CombatComponent.Fire` (`self.CombatComponent`))))

(event `InputAction|Interact`
  (params (Key :type "Key Structure"))
  ;[1 0.1042 0.1042] Player actions
  (:`Pressed`
    (`/Game/SpaceBlaster/Core/Components/BP_InteractionComponent.Interact` (`self.BP_InteractionComponent`))))

(fn `Kill`
  (params (A :type "Float (double-precision)"))
  (if (<= A 0.0)
    (`self.K2_DestroyActor` (`/Game/SpaceBlaster/Combat/BP_CombatComponent.CurrentWeapon` (`self.CombatComponent`)))
    (`self.K2_DestroyActor`)))

(fn `UserConstructionScript`)