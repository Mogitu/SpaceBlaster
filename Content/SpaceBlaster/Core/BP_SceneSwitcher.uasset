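; BP_SceneSwitcher is a trigger volume in SpaceBlaster that ends the level when the player enters it.
; When the player pawn overlaps its Box, it creates and shows a WBP_EndOfLevel widget, disables character movement and switches input to UI only.
; It passes its LevelToSwitchTo value to the widget's LevelToChange, leaving the level change to that widget.
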(event `self.Box.OnComponentBeginOverlap`
  (params (OverlappedComponent :type "PrimitiveComponent Object Reference") (OtherActor :type "Actor Object Reference") (OtherComp :type "PrimitiveComponent Object Reference") (OtherBodyIndex :type Integer) (bFromSweep :type Boolean) (SweepResult :type "HitResult Structure (by ref)"))
  (bind _returnvalue (`GameplayStatics.GetPlayerController` 0))
  (if (== OtherActor (`GameplayStatics.GetPlayerPawn` 0))
    (bind _returnvalue_2 (`|CreateWidget` "/Game/SpaceBlaster/UI/WBP_EndOfLevel.WBP_EndOfLevel_C" _returnvalue))
    (`CharacterMovementComponent.DisableMovement` (`Character.CharacterMovement` (`GameplayStatics.GetPlayerCharacter` 0)))
    (`UserWidget.AddToViewport` _returnvalue_2 0)
    (`WidgetBlueprintLibrary.SetInputMode_UIOnlyEx` _returnvalue _returnvalue_2)
    (set `/Game/SpaceBlaster/UI/WBP_EndOfLevel.LevelToChange` (`self.LevelToSwitchTo`) _returnvalue_2)))

(fn `UserConstructionScript`)