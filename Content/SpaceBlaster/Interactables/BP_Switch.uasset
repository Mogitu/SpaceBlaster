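; BP_Switch is an interactable switch that forwards an Interact event to a list of linked Interactables, optionally gated by required gameplay tags.
; On interaction it plays a sound, then checks the instigator's BP_InventoryComponent for all RequiredTags, printing a message if any are missing.
; With no required tags, or an instigator lacking that component, the gate is bypassed and every linked actor is triggered.
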(event `/Game/SpaceBlaster/Interactables/BPI_Interaction.Interact`
  (params (Instigator :type "Actor Object Reference"))
  (bind _returnvalue (`self.GetComponentByClass` Instigator "/Game/SpaceBlaster/Core/Components/BP_InventoryComponent.BP_InventoryComponent_C"))
  (`GameplayStatics.PlaySoundAtLocation` (`self.InteractSound`) (`self.K2_GetActorLocation`) (struct) 1.0 1.0 0.0 null null null null)
  (if (> (`BlueprintGameplayTagLibrary.GetNumGameplayTagsInContainer` (`self.RequiredTags`)) 0)
    (`/Engine/EditorBlueprintResources/StandardMacros.IsValid` _returnvalue
      (:`Is Valid`
        (if (`BlueprintGameplayTagLibrary.HasAllTags` (`/Game/SpaceBlaster/Core/Components/BP_InventoryComponent.CollectedInventoryTags` _returnvalue) (`self.RequiredTags`))
          (for _array_element (`self.Interactables`) :!label _label
            (`/Game/SpaceBlaster/Interactables/BPI_Interaction.Interact` _array_element Instigator))
          (else
            (`KismetSystemLibrary.PrintString` "Dont have the tags!"))))
      (:`Is Not Valid`
        (goto _label)))
    (else
      (goto _label))))

(fn `UserConstructionScript`
  (`parent.UserConstructionScript`))