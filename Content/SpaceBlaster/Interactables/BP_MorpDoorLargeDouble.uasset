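; Interactable large double door in SpaceBlaster that opens by animating a morph target on its skeletal mesh.
; On Interact it plays a sound at its location and runs the OpenDoor timeline, whose Morph track drives the named morph target each update.
; When the timeline finishes, the Box collision is disabled; the graph has no closing logic.
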(event `/Game/SpaceBlaster/Interactables/BPI_Interaction.Interact`
  (params (Instigator :type "Actor Object Reference"))
  (`GameplayStatics.PlaySoundAtLocation` (`self.InteractSound`) (`self.K2_GetActorLocation`) (struct) 1.0 1.0 0.0 null null null null)
  (bind (_direction _morph) (`Timeline|OpenDoor`)
    (:`Update`
      (`SkeletalMeshComponent.SetMorphTarget` (`self.SkeletalMesh`) (`self.Morph Target Name`) _morph true))
    (:`Finished`
      (`PrimitiveComponent.SetCollisionEnabled` (`self.Box`) "NoCollision"))))

(fn `UserConstructionScript`
  (`parent.UserConstructionScript`))