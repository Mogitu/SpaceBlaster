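; Combat component for a Character that manages its weapons: firing, swapping, ammo grants and dropping.
; On BeginPlay it spawns the starter weapon hidden on a mesh socket, adds it to the collection and equips it.
; Swapping shows the first collected weapon that differs from the current one, with sound and a change notification.
; Ammo goes to the matching weapon type; dropping enables physics on the current weapon's mesh.
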(event `self.ReceiveBeginPlay`
  (bind _ascharacter (cast `Character` (`self.GetOwner`)))
  (set `self.OwningPlayer` _ascharacter)
  (`self.AddWeapon` (`self.StarterWeapon`))
  (`self.ChangeWeapon`))

(fn `AddWeapon`
  (params (WeaponToAdd :type "/Game/SpaceBlaster/Combat/BPA_Weapon Class Reference"))
  (bind _spawnedweapon (`self.SpawnWeapon` WeaponToAdd))
  (`KismetArrayLibrary.Array_AddUnique` (`self.CollectedWeapons`) _spawnedweapon))

(fn `ChangeWeapon`
  (if (`KismetSystemLibrary.IsValid` (`self.CurrentWeapon`))
    (for _array_element (`self.CollectedWeapons`)
      (if (!= _array_element (`self.CurrentWeapon`))
        (`Actor.SetActorHiddenInGame` (`self.CurrentWeapon`) true)
        (`self.ReleaseTrigger`)
        (bind _output_get (set `self.CurrentWeapon` _array_element))
        (`Actor.SetActorHiddenInGame` _output_get false)
        (`self.PlaySwapSound`)
        (`self.OnChangeWeapon` _output_get)
        (break)))
    (else
      (bind _output_get_2 (set `self.CurrentWeapon` (`|GetArrayItem` (`self.CollectedWeapons`))))
      (`Actor.SetActorHiddenInGame` _output_get_2 false)
      (`self.OnChangeWeapon` _output_get_2))))

(fn `DropWeapon`
  (bind _weaponmesh (`/Game/SpaceBlaster/Combat/BPA_Weapon.WeaponMesh` (`self.CurrentWeapon`)))
  (`self.ReleaseTrigger`)
  (`PrimitiveComponent.SetCollisionEnabled` _weaponmesh "PhysicsOnly")
  (`PrimitiveComponent.SetSimulatePhysics` _weaponmesh true)
  (`Actor.K2_DetachFromActor` (`self.OwningPlayer`) "KeepWorld" "KeepWorld" "KeepWorld"))

(fn `GetSpawnTransform`
  (returns (ReturnValue :type "Transform Structure"))
  (return (`SceneComponent.GetSocketTransform` (`Character.Mesh` (`GameplayStatics.GetPlayerCharacter` 0)) (`self.WeaponSocketName`) "RTS_Actor")))

(fn `GrantAmmoToWeapon`
  (params (WeaponType :type "/Game/SpaceBlaster/Combat/E_WeaponType Enum" :default "NewEnumerator0") (AmmToGrant :type Integer))
  ;[1 1 1] Only grant the weapon of the selected type the ammo
  (for _array_element (`self.CollectedWeapons`)
    (bind _weapontype (`/Game/SpaceBlaster/Combat/BP_WeaponDataAsset.WeaponType` (`/Game/SpaceBlaster/Combat/BPA_Weapon.WeaponData` _array_element)))
    (if (`|EnumEquality` _weapontype WeaponType)
      (`/Game/SpaceBlaster/Combat/BPA_Weapon.GrantAmmo` _array_element AmmToGrant (`|EnumEquality` _weapontype (`/Game/SpaceBlaster/Combat/BP_WeaponDataAsset.WeaponType` (`/Game/SpaceBlaster/Combat/BPA_Weapon.WeaponData` (`self.CurrentWeapon`)))))
      (break))))

(fn `PlaySwapSound`
  (`GameplayStatics.PlaySoundAtLocation` (`self.WeaponChangeSound`) (`Actor.K2_GetActorLocation` (`self.GetOwner`)) (struct) 1.0 1.0 0.0 null null null null))

(fn `PullTrigger`
  (bind _currentweapon (`self.CurrentWeapon`))
  ;[1 1 1] Fire the current weapon if it is valid
  (`/Engine/EditorBlueprintResources/StandardMacros.IsValid` _currentweapon
    (:`Is Valid`
      (`/Game/SpaceBlaster/Combat/BPA_Weapon.StartFire` _currentweapon (`Actor.GetActorForwardVector` (`self.OwningPlayer`))))))

(fn `ReleaseTrigger`
  (`/Game/SpaceBlaster/Combat/BPA_Weapon.StopFire` (`self.CurrentWeapon`)))

(fn `SpawnWeapon`
  (params (WeaponClass :type "/Game/SpaceBlaster/Combat/BPA_Weapon Class Reference"))
  (returns (SpawnedWeapon :type "/Game/SpaceBlaster/Combat/BPA_Weapon Object Reference"))
  (locals (WeaponInstance :type "/Game/SpaceBlaster/Combat/BPA_Weapon Object Reference"))
  (bind _owningplayer (`self.OwningPlayer`))
  (bind _returnvalue (`|SpawnActorFromClass` WeaponClass (`self.GetSpawnTransform`) "AlwaysSpawn" "OverrideRootScale" _owningplayer _owningplayer))
  (bind _output_get (set `local.WeaponInstance` _returnvalue))
  (`Actor.SetActorHiddenInGame` _output_get true)
  (`Actor.K2_AttachToComponent` _output_get (`Character.Mesh` (`self.OwningPlayer`)) (`self.WeaponSocketName`) "SnapToTarget" "SnapToTarget" "SnapToTarget" true)
  (return (`local.WeaponInstance`)))