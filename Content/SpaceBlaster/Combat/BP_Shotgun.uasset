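; BP_Shotgun is a SpaceBlaster combat weapon that fires a fan of projectiles with each shot.
; Fire checks CanFire, deducts the ammo cost once per shot, or prints an out-of-ammo message when the check fails.
; It rotates the fire direction around the Z axis in steps of Angle divided by ProjectileCount, starting at minus half Angle, so the fan stops one step short of the positive edge.
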(fn `Fire`
  (params (FireDirection :type "Vector Structure"))
  (locals (RotatedDirection :type "Vector Structure") (StartAngle :type "Float (double-precision)") (Offset :type "Float (double-precision)"))
  (if (`self.CanFire`)
    (`self.UpdateAmmo` (`self.AmmoCost`))
    (set `local.StartAngle` (/ (`self.Angle`) 2.0))
    (set `local.Offset` (/ (`self.Angle`) (`self.ProjectileCount`)))
    (for _ (range (`self.ProjectileCount`))
      (`self.SpawnProjectile` (`KismetMathLibrary.RotateAngleAxis` FireDirection (- 0.0 (`local.StartAngle`)) (0.0 0.0 1.0)))
      (set `local.StartAngle` (- (`local.StartAngle`) (`local.Offset`))))
    (else
      (`KismetSystemLibrary.PrintString` "Out of ammo"))))

(fn `UserConstructionScript`
  (`parent.UserConstructionScript`))