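; BP_BlueKey is a pickup in SpaceBlaster, named as a blue key, that grants items to whoever picks it up.
; On pickup, it looks for a BP_InventoryComponent on the instigator and, if one exists, adds its GrantTags to that inventory.
; It has no other active logic of its own, as the stock events are disabled and the construction script only calls the parent.
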(event `/Game/SpaceBlaster/Pickups/BPI_Pickup.OnPickup`
  (params (Instigator :type "Actor Object Reference"))
  (bind _returnvalue (`self.GetComponentByClass` Instigator "/Game/SpaceBlaster/Core/Components/BP_InventoryComponent.BP_InventoryComponent_C"))
  (`/Engine/EditorBlueprintResources/StandardMacros.IsValid` _returnvalue
    (:`Is Valid`
      (`/Game/SpaceBlaster/Core/Components/BP_InventoryComponent.AddItems` _returnvalue (`self.GrantTags`)))))

(fn `UserConstructionScript`
  (`parent.UserConstructionScript`))