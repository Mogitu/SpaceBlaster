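; BP_Projectile is a projectile actor that applies its Damage value to actors it overlaps.
; On BeginPlay its CollisionSphere ignores the instigator when moving, and the overlap handler also filters the instigator out.
; An overlapped actor with a BP_HealthComponent receives Damage through ApplyHealthChange, then the projectile destroys itself.
; Overlaps with actors lacking that component leave the projectile alive.
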(event `self.ReceiveBeginPlay`
  (`PrimitiveComponent.IgnoreActorWhenMoving` (`self.CollisionSphere`) (`self.GetInstigator`) true))

(event `self.CollisionSphere.OnComponentBeginOverlap`
  (params (OverlappedComponent :type "PrimitiveComponent Object Reference") (OtherActor :type "Actor Object Reference") (OtherComp :type "PrimitiveComponent Object Reference") (OtherBodyIndex :type Integer) (bFromSweep :type Boolean) (SweepResult :type "HitResult Structure (by ref)"))
  (bind _returnvalue (`self.GetComponentByClass` OtherActor "/Game/Blueprint/Components/BP_HealthComponent.BP_HealthComponent_C"))
  (if (!= OtherActor (`self.GetInstigator`))
    (`/Engine/EditorBlueprintResources/StandardMacros.IsValid` _returnvalue
      (:`Is Valid`
        (`/Game/Blueprint/Components/BP_HealthComponent.ApplyHealthChange` _returnvalue (`self.Damage`))
        (`self.K2_DestroyActor`)))))

(fn `UserConstructionScript`)