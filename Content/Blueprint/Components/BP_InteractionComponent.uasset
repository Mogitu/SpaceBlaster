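; Actor component that detects a nearby interactable object for its owner and lets it trigger an interaction.
; Each tick, a sphere trace at the owner's location stores a hit actor implementing BP_InteractionInterface, if none is stored.
; It clears that actor only when the trace hits nothing, firing OnUpdateInteractable on either change.
; Interact sends InteractMessage to the stored actor.
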(event `self.ReceiveTick`
  (params (DeltaSeconds :type "Float (single-precision)"))
  (`self.FindInteractable`))

(fn `FindInteractable`
  (bind _returnvalue (`Actor.K2_GetActorLocation` (`self.GetOwner`)))
  (bind (_outhit _returnvalue_2) (`KismetSystemLibrary.SphereTraceSingleForObjects` _returnvalue _returnvalue 100.0 (`self.Object Types`)))
  (if _returnvalue_2
    (if (`KismetSystemLibrary.DoesImplementInterface` (`.HitActor` (`GameplayStatics.BreakHitResult` _outhit)) "/Game/Blueprint/Components/BP_InteractionInterface.BP_InteractionInterface_C")
      (`/Engine/EditorBlueprintResources/StandardMacros.IsValid` (`self.CurrentInterActable`)
        (:`Is Not Valid`
          (set `self.CurrentInterActable` (`.HitActor` (`GameplayStatics.BreakHitResult` _outhit)))
          (`self.OnUpdateInteractable` true))))
    (else
      (`/Engine/EditorBlueprintResources/StandardMacros.IsValid` (`self.CurrentInterActable`)
        (:`Is Valid`
          (set `self.CurrentInterActable` null)
          (`self.OnUpdateInteractable` false))))))

(fn `Interact`
  (bind _currentinteractable (`self.CurrentInterActable`))
  (`/Engine/EditorBlueprintResources/StandardMacros.IsValid` _currentinteractable
    (:`Is Valid`
      (message `/Game/Blueprint/Components/BP_InteractionInterface.Interact` _currentinteractable))))